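; BP_ConductingLine is a spline guide line that detects when the conducting baton's tip comes close to it.
; On BeginPlay it caches the BP_ConductingBaton actor.
; Each Tick it measures from the tip to the closest spline point and latches IsTrace once within AcceptableDistance, which ends further checks.
; Timeline-driven point movement, spline mesh construction and debug spheres are present but disconnected.
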(event EventBeginPlay
  (bind _returnvalue (Actor|GetActorOfClass "/Game/develop/Takeuchi/BP_/BP_ConductingBaton.BP_ConductingBaton_C"))
  (Variables|Default|SetBaton _returnvalue))

(event EventTick
  (params (DeltaSeconds :type Float%20%28single-precision%29))
  (bind _baton (Variables|Default|GetBaton))
  (if (not (Variables|Default|GetIsTrace))
    (Utilities|IsValid _baton
      (:Is%20Valid
        (bind _output_get (Variables|Default|SetBatonLocation (Transformation|GetWorldLocation (Variables|/Game/develop/Takeuchi/BP_/BP_ConductingBaton.BP_ConductingBaton_C|GetBatonTip _baton))))
        (bind _output_get_2 (Variables|Default|SetClosestLocationOnSpline (Spline|FindLocationClosesttoWorldLocation (Variables|Default|GetSpline) _output_get "World")))
        (bind _output_get_3 (Variables|Default|SetCurrentDistance (Math|Vector|Distance(Vector) (Variables|Default|GetBatonLocation) (Variables|Default|GetClosestLocationOnSpline))))
        (if (<= _output_get_3 (Variables|Default|GetAcceptableDistance))
          (Utilities|FlowControl|DoOnce false
            (:Completed
              (Variables|Default|SetIsTrace true))))))))

(fn ConstructionScript)