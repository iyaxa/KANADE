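; BP_ConductingBaton is a conducting baton actor with a baton mesh, a tip component and a GrabComponent for picking it up.
; Its grab and drop events are empty; disconnected nodes would tint the baton's dynamic material green when held and white when released, with debug prints.
; An unused node chain would project the tip onto the closest point of the ConductingLine spline.
; The construction script is empty, so the graphs currently run no logic.
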(event OnDropped(GrabComponent)
  ;[0.15 0.15 0.15 0.5] Grabされたら色を変える
)

(event OnGrabbed(GrabComponent)
  ;[0.15 0.15 0.15 0.5] Grabされたら色を変える
)

(fn ConstructionScript)