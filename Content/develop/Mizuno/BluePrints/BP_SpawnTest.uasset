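; BP_SpawnTest is a test Blueprint that triggers timed creation at its own transform.
; Tick accumulates delta time until it exceeds Interval, then prints a debug string and resets the timer.
; At each interval it calls Create on the NewVar reference, passing the actor's transform and a Texture variable.
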(event EventBeginPlay)

(event Collision|EventActorBeginOverlap
  (params (OtherActor :type Actor%20Object%20Reference)))

(event EventTick
  (params (DeltaSeconds :type Float%20%28single-precision%29))
  (bind _output_get (Variables|Default|Settime (+ DeltaSeconds (Variables|Default|Gettime))))
  (if (> _output_get (Variables|Default|Getinterval))
    (Development|PrintString "W")
    (Default|Create (Variables|Default|GetNewVar) (Transformation|GetActorTransform) (Variables|Default|Gettexture))
    (Variables|Default|Settime 0.0)))

(fn ConstructionScript)