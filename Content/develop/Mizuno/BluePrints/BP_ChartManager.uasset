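; Chart manager actor that drives timed note spawning for a six-lane chart, apparently for a rhythm game.
; On BeginPlay it shows the life widget and reads the note DataTable rows into per-lane boolean arrays, exposed through getters.
; Tick accumulates and prints elapsed time, and at each interval step within the chart length calls NewCreate on every registered spawner, observer-style.
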(event EventBeginPlay
  (bind _returnvalue (UserInterface|CreateWidget "/Game/develop/Mizuno/BluePrints/WBP_Life.WBP_Life_C"))
  (bind _output_get (Variables|Default|SetWBP _returnvalue))
  (UserInterface|Viewport|AddtoViewport _output_get 0)
  (bind _outrownames (DataTable|GetDataTableRowNames "/Game/develop/Mizuno/DataAsset/NoteDataTable.NoteDataTable"))
  (for _array_element _outrownames
    (bind _returnvalue_2 (Utilities|GetDataTableRow (Variables|Default|Getdatatable) _array_element)
      (:then
        (CallFunction|AddLaneSpawnTime (.Lane1 (Utilities|Struct|BreakST_ChartRow _returnvalue_2)) (Variables|Default|GetLane1SpawnTimes))
        (CallFunction|AddLaneSpawnTime (.Lane2 (Utilities|Struct|BreakST_ChartRow _returnvalue_2)) (Variables|Default|GetLane2SpawnTimes))
        (CallFunction|AddLaneSpawnTime (.Lane3 (Utilities|Struct|BreakST_ChartRow _returnvalue_2)) (Variables|Default|GetLane3SpawnTimes))
        (CallFunction|AddLaneSpawnTime (.Lane4 (Utilities|Struct|BreakST_ChartRow _returnvalue_2)) (Variables|Default|GetLane4SpawnTimes))
        (CallFunction|AddLaneSpawnTime (.Lane5 (Utilities|Struct|BreakST_ChartRow _returnvalue_2)) (Variables|Default|GetLane5SpawnTimes))
        (CallFunction|AddLaneSpawnTime (.Lane6 (Utilities|Struct|BreakST_ChartRow _returnvalue_2)) (Variables|Default|GetLane6SpawnTimes))
        (Variables|Default|SetLane1Index (+ (Variables|Default|GetLane1Index) 1))
        (Variables|Default|SetTime 0.0)))))

(event Collision|EventActorBeginOverlap
  (params (OtherActor :type Actor%20Object%20Reference)))

(event EventTick
  (params (DeltaSeconds :type Float%20%28single-precision%29))
  (if (not (Variables|Default|Geta))
    (bind _output_get (Variables|Default|SetTime (+ DeltaSeconds (Variables|Default|GetTime))))
    (Development|PrintString (Utilities|String|ToString(Float) _output_get))
    (if (> _output_get (* (Variables|Default|GetIntarvalTime) (Variables|Default|Getindex)))
      (if (>= (Utilities|Array|Length (Variables|Default|GetLane1SpawnTimes)) (Variables|Default|Getindex))
        (Variables|Default|Seta true)
        (for _array_element (Variables|Default|GetObserver)
          (Default|NewCreate _array_element))
        (Variables|Default|Setindex (+ (Variables|Default|Getindex) 1))
        (Variables|Default|Seta false)))))

(fn ConstructionScript)

(fn AddLaneSpawnTime
  (params (NewParam :type Integer) (NewParam1 :type Array%20of%20Booleans))
  (Utilities|Array|Add NewParam1 (Math|Conversions|ToBoolean(Integer) NewParam))
  (return))

(fn GetLaneSpawnTime
  (params (LaneNum :type Integer))
  (switch int LaneNum
    (:1
      (return (Variables|Default|GetLane1SpawnTimes)))
    (:2
      (return (Variables|Default|GetLane2SpawnTimes)))
    (:3
      (return (Variables|Default|GetLane3SpawnTimes)))
    (:4
      (return (Variables|Default|GetLane4SpawnTimes)))
    (:5
      (return (Variables|Default|GetLane5SpawnTimes)))
    (:6
      (return (Variables|Default|GetLane6SpawnTimes)))))

(fn GetTime
  (return (Variables|Default|GetTime)))

(fn SetNoteSpawner
  (params (NewParam :type BP%20Note%20Spawner%20Object%20Reference))
  (Utilities|Array|Add (Variables|Default|GetObserver) NewParam))