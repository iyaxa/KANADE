(event EventBeginPlay
  (Utilities|FlowControl|Delay 0.2)
  (bind _newparam (Default|GetLaneSpawnTime (Variables|Default|GetChartManager) (Variables|Default|GetLane)))
  (Variables|Default|SetSpawnTime _newparam)
  (Default|SetNoteSpawner (Variables|Default|GetChartManager) self))

(event Collision|EventActorBeginOverlap
  (params (OtherActor :type Actor%20Object%20Reference)))

(event EventTick
  (params (DeltaSeconds :type Float%20%28single-precision%29)))

(fn ConstructionScript)

(fn Create
  (params (CreateTransform :type Transform) (Texture :type Texture%202D%20Object%20Reference))
  (bind _returnvalue (Game|SpawnActorfromClass (Variables|Default|GetNote) (Math|Transform|MakeTransform (.location CreateTransform) (Math|Conversions|RotationFromXVector (- (Transformation|GetActorLocation (Variables|Default|Gettarget)) (.location CreateTransform))) (.scale CreateTransform)) "Undefined" "MultiplyWithRoot" 0 0))
  (Variables|/Game/develop/Mizuno/BluePrints/BP_Note.BP_Note_C|Setplayer _returnvalue (Variables|Default|Gettarget))
  (if (Utilities|IsValid Texture)
    (Rendering|Components|Sprite|SetSprite (Variables|/Game/develop/Mizuno/BluePrints/BP_Note.BP_Note_C|GetBillboard _returnvalue) Texture)
    (Development|PrintString "Create")
    (else
      (Rendering|Components|Sprite|SetSprite (Variables|/Game/develop/Mizuno/BluePrints/BP_Note.BP_Note_C|GetBillboard _returnvalue) "/Game/Characters/MannequinsXR/Textures/Shared/T_UE_Logo_M.T_UE_Logo_M")))
  (Variables|/Script/Engine.ProjectileMovementComponent|SetHomingTargetComponent (Variables|/Game/develop/Mizuno/BluePrints/BP_Note.BP_Note_C|GetProjectileMovement _returnvalue) (Variables|/Script/Engine.Actor|GetRootComponent (Variables|Default|Gettarget)))
  (Variables|/Script/Engine.ProjectileMovementComponent|SetbIsHomingProjectile (Variables|/Game/develop/Mizuno/BluePrints/BP_Note.BP_Note_C|GetProjectileMovement _returnvalue) true)
  (Variables|/Game/develop/Mizuno/BluePrints/BP_Note.BP_Note_C|SetWBP _returnvalue (Variables|Default|GetWBP)))

(fn NewCreate
  (bind _returnvalue (Transformation|GetActorLocation))
  (if (Utilities|Array|Get(acopy) (Variables|Default|GetSpawnTime) (Variables|Default|Getindex))
    (Variables|Default|Setindex (+ (Variables|Default|Getindex) 1))
    (Game|SpawnActorfromClass (Variables|Default|GetNote) (Math|Transform|MakeTransform _returnvalue (Math|Conversions|RotationFromXVector _returnvalue)) "Undefined" "MultiplyWithRoot" 0 0)
    (else
      (Variables|Default|Setindex (+ (Variables|Default|Getindex) 1)))))